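; Board actor for the Yinsh board game that runs match state, turns and move rules on top of a WBP_YinshBoard widget.
; On widget construct it indexes the space widgets into a map of rows by letter and number.
; Clicks preview annulus deployment, then annulus moves that leave spirits, validated along three axes for blockers and spirit jumps.
; Confirming a move logs the turn action and passes the turn.
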(event Custom|OnConstruct_Event_0
  (CallFunction|SetUpBoardData)
  (CallFunction|PrintBoard))

(event Custom|StartGameDispatcher_Event_0
  (params (YinshGameType :type YinshType%20Enum :default "NewEnumerator0"))
  (Variables|Default|SetGameType YinshGameType)
  (Variables|Default|SetbGameInProgress true)
  (Default|OnStartGame (CallFunction|GetYinshBoard) "NewEnumerator0")
  (CallFunction|SetCurrentTurn "NewEnumerator0"))

(event Custom|OnResetMove)

(event EventBeginPlay
  (bind _aswbp_yinsh_board (Utilities|Casting|CastToWBP_YinshBoard (UserInterface|GetUserWidgetObject (Variables|Default|GetWidget))))
  (EventDispatchers|AssignOnConstruct _aswbp_yinsh_board (delegate Custom|OnConstruct_Event_0))
  (EventDispatchers|AssignStartGameDispatcher _aswbp_yinsh_board (delegate Custom|StartGameDispatcher_Event_0)))

(event Collision|EventActorBeginOverlap
  (params (OtherActor :type Actor%20Object%20Reference)))

(event EventTick
  (params (DeltaSeconds :type Float%20%28single-precision%29)))

(fn ConstructionScript)

(fn SetUpBoardData
  (bind _aswbp_yinsh_board (Utilities|Casting|CastToWBP_YinshBoard (UserInterface|GetUserWidgetObject (Variables|Default|GetWidget))))
  (Variables|/Game/Yinsh/Widgets/WBP_YinshBoard.WBP_YinshBoard_C|SetYinshBoardActor _aswbp_yinsh_board self)
  (bind _spacewidgets (Default|GetYinshSpaceWidgets _aswbp_yinsh_board))
  (Variables|Default|SetYinshSpaceWidgets _spacewidgets)
  (for _array_element _spacewidgets
    (Utilities|Array|Clear (LocalVariables|GetLocalSpaceArray))
    (if (.ReturnValue (Utilities|Map|Find (Variables|Default|GetYinshMap) (Variables|/Game/Yinsh/Widgets/WBP_YinshSpace.WBP_YinshSpace_C|GetLetterAxis _array_element)))
      (LocalVariables|SetLocalSpaceArray (Utilities|Struct|BreakYinshRow (.Value (Utilities|Map|Find (Variables|Default|GetYinshMap) (Variables|/Game/Yinsh/Widgets/WBP_YinshSpace.WBP_YinshSpace_C|GetLetterAxis _array_element)))))
      (Utilities|Array|SetArrayElem (LocalVariables|GetLocalSpaceArray) (- (Variables|/Game/Yinsh/Widgets/WBP_YinshSpace.WBP_YinshSpace_C|GetNumberAxis _array_element) 1) _array_element true)
      (Utilities|Map|Add (Variables|Default|GetYinshMap) (Variables|/Game/Yinsh/Widgets/WBP_YinshSpace.WBP_YinshSpace_C|GetLetterAxis _array_element) (Utilities|Struct|MakeYinshRow (LocalVariables|GetLocalSpaceArray)))
      (else
        (Utilities|Array|SetArrayElem (LocalVariables|GetLocalSpaceArray) (- (Variables|/Game/Yinsh/Widgets/WBP_YinshSpace.WBP_YinshSpace_C|GetNumberAxis _array_element) 1) _array_element true)
        (Utilities|Map|Add (Variables|Default|GetYinshMap) (Variables|/Game/Yinsh/Widgets/WBP_YinshSpace.WBP_YinshSpace_C|GetLetterAxis _array_element) (Utilities|Struct|MakeYinshRow (LocalVariables|GetLocalSpaceArray)))))))

(fn PrintBoard
  (bind _keys (Utilities|Map|Keys (Variables|Default|GetYinshMap)))
  (for _array_element _keys
    (if (.ReturnValue (Utilities|Map|Find (Variables|Default|GetYinshMap) _array_element))
      (for _array_element_2 (Utilities|Struct|BreakYinshRow (.Value (Utilities|Map|Find (Variables|Default|GetYinshMap) _array_element)))
        (Utilities|IsValid _array_element_2
          (:Is%20Valid
            (LocalVariables|SetLocalRowString (Utilities|String|Append (LocalVariables|GetLocalRowString) "  " (Utilities|String|Append (Utilities|String|EnumtoString (Variables|/Game/Yinsh/Widgets/WBP_YinshSpace.WBP_YinshSpace_C|GetLetterAxis _array_element_2)) (Utilities|String|ToString(Integer) (Variables|/Game/Yinsh/Widgets/WBP_YinshSpace.WBP_YinshSpace_C|GetNumberAxis _array_element_2))))))))
      (Development|PrintString (LocalVariables|GetLocalRowString) true true "(R=0.000000,G=0.660000,B=1.000000,A=1.000000)" 6e+01)
      (LocalVariables|SetLocalRowString ""))))

(fn OnRepCurrentTurn
  (CallFunction|OnCurrentTurnSet))

(fn OnRepGameType)

(fn SetCurrentTurn
  (params (InTurn :type YinshTurnState%20Enum :default "NewEnumerator0"))
  (Variables|Default|SetCurrentTurn InTurn)
  (CallFunction|OnCurrentTurnSet))

(fn OnCurrentTurnSet
  (bind _outyinshboard (CallFunction|GetYinshBoard))
  (Utilities|IsValid _outyinshboard
    (:Is%20Valid
      (Default|OnCurrentTurnSet _outyinshboard (Variables|Default|GetCurrentTurn)))))

(fn GetYinshBoard
  (bind _aswbp_yinsh_board (Utilities|Casting|CastToWBP_YinshBoard (UserInterface|GetUserWidgetObject (Variables|Default|GetWidget))))
  (return _aswbp_yinsh_board))

(fn OnVinshSpaceClicked
  (params (VinshSpace :type WBP%20Yinsh%20Space%20Object%20Reference))
  (bind _selectedspacearray (Variables|Default|GetSelectedSpaceArray))
  (bind _selectedspacearray_2 (Variables|Default|GetSelectedSpaceArray))
  (bind _output (Utilities|Array|Get(acopy) _selectedspacearray_2))
  (LocalVariables|SetLocalVinshSpace VinshSpace)
  (if (Variables|Default|GetbGameInProgress)
    (if (< (Utilities|Select :Index (Variables|Default|GetCurrentTurn) :NewEnumerator0 (Variables|Default|GetWhiteAnnulusDeployed) :NewEnumerator1 (Variables|Default|GetBlackAnnulusDeployed)) 5) ; Annulus Deploy Phase
      (if (Utilities|Enum|Equal(Enum) (Variables|/Game/Yinsh/Widgets/WBP_YinshSpace.WBP_YinshSpace_C|GetSpaceState (LocalVariables|GetLocalVinshSpace)) "NewEnumerator0")
        ;[1 1 1] Deploy Annulus Phase
        (Utilities|FlowControl|Sequence
          (:then_0
            (if (> (Utilities|Array|Length (Variables|Default|GetSelectedSpaceArray)) 0)
              (Default|SetSpaceState (Utilities|Array|Get(acopy) (Variables|Default|GetSelectedSpaceArray)) "NewEnumerator0")))
          (:then_1
            (Utilities|Array|Clear (Variables|Default|GetSelectedSpaceArray))
            (Default|SetSpaceState (LocalVariables|GetLocalVinshSpace) (Utilities|Select :Index (Variables|Default|GetCurrentTurn) :NewEnumerator0 "NewEnumerator1" :NewEnumerator1 "NewEnumerator4"))
            (Variables|Default|SetCurrentTurnAction (Utilities|Struct|MakeYinshTurnActionStruct (Variables|Default|GetCurrentTurn) (Utilities|Array|MakeArray (Utilities|Struct|MakeYinshSpaceActionStruct "NewEnumerator0" (Utilities|Struct|MakeYinshSpaceStruct (LocalVariables|GetLocalVinshSpace) (Variables|/Game/Yinsh/Widgets/WBP_YinshSpace.WBP_YinshSpace_C|GetLetterAxis (LocalVariables|GetLocalVinshSpace)) (Variables|/Game/Yinsh/Widgets/WBP_YinshSpace.WBP_YinshSpace_C|GetNumberAxis (LocalVariables|GetLocalVinshSpace))))))))
          (:then_2
            (Utilities|Array|Add (Variables|Default|GetSelectedSpaceArray) (LocalVariables|GetLocalVinshSpace)))))
      (else
        (Utilities|FlowControl|Sequence
          (:then_0
            ;[1 1 1] Select Annulus Space
            (bind _localvinshspace (LocalVariables|GetLocalVinshSpace)
              (:then
                (if (Utilities|Select :Index (Variables|Default|GetCurrentTurn) :NewEnumerator0 (Utilities|Enum|Equal(Enum) (Variables|/Game/Yinsh/Widgets/WBP_YinshSpace.WBP_YinshSpace_C|GetSpaceState _localvinshspace) "NewEnumerator1") :NewEnumerator1 (Utilities|Enum|Equal(Enum) (Variables|/Game/Yinsh/Widgets/WBP_YinshSpace.WBP_YinshSpace_C|GetSpaceState _localvinshspace) "NewEnumerator4")) ; If we selected an annulus
                  ;;[1 1 1] Selecting annulus to move
                  (Utilities|FlowControl|Sequence
                    (:then_0
                      (if (Utilities|Array|IsValidIndex _selectedspacearray 1)
                        (if (== (Utilities|Array|Get(acopy) _selectedspacearray 1) (LocalVariables|GetLocalVinshSpace)) ; If we selected teh annulus we just put down, return
                          (return))))
                    (:then_1
                      (for (_array_element _array_index) (Variables|Default|GetSelectedSpaceArray)
                        (if (== _array_index 0)
                          (Default|SetSpaceState _array_element (Utilities|Select :Index (Variables|Default|GetCurrentTurn) :NewEnumerator0 "NewEnumerator1" :NewEnumerator1 "NewEnumerator4"))
                          (else
                            (Default|SetSpaceState _array_element "NewEnumerator0"))))
                      (Utilities|Array|Clear (Variables|Default|GetSelectedSpaceArray))
                      (Utilities|Array|Add (Variables|Default|GetSelectedSpaceArray) (LocalVariables|GetLocalVinshSpace))
                      (Default|SetSpaceState (LocalVariables|GetLocalVinshSpace) (Utilities|Select :Index (Variables|Default|GetCurrentTurn) :NewEnumerator0 "NewEnumerator1" :NewEnumerator1 "NewEnumerator4"))
                      (return)))
                  (else
                    ;;[1 1 1] Move selected annulus to vacant space, spawn spirit
                    (if (> (Utilities|Array|Length (Variables|Default|GetSelectedSpaceArray)) 0)
                      (if (Utilities|Enum|Equal(Enum) (Variables|/Game/Yinsh/Widgets/WBP_YinshSpace.WBP_YinshSpace_C|GetSpaceState (LocalVariables|GetLocalVinshSpace)) "NewEnumerator0")
                        (bind _bvalid (CallFunction|IsValidAnnulusMove (Utilities|Array|Get(acopy) (Variables|Default|GetSelectedSpaceArray)) (LocalVariables|GetLocalVinshSpace)))
                        (if _bvalid
                          (Utilities|FlowControl|Sequence
                            (:then_0
                              (if (Utilities|Array|IsValidIndex (Variables|Default|GetSelectedSpaceArray) 1)
                                (Default|SetSpaceState (Utilities|Array|Get(acopy) (Variables|Default|GetSelectedSpaceArray) 1) "NewEnumerator0")
                                (Utilities|Array|RemoveIndex (Variables|Default|GetSelectedSpaceArray) 1)))
                            (:then_1
                              (Default|SetSpaceState (Utilities|Array|Get(acopy) (Variables|Default|GetSelectedSpaceArray)) (Utilities|Select :Index (Variables|Default|GetCurrentTurn) :NewEnumerator0 "NewEnumerator2" :NewEnumerator1 "NewEnumerator5"))
                              (Default|SetSpaceState (LocalVariables|GetLocalVinshSpace) (Utilities|Select :Index (Variables|Default|GetCurrentTurn) :NewEnumerator0 "NewEnumerator1" :NewEnumerator1 "NewEnumerator4"))
                              (Utilities|Array|Add (Variables|Default|GetSelectedSpaceArray) (LocalVariables|GetLocalVinshSpace))
                              (Variables|Default|SetCurrentTurnAction (Utilities|Struct|MakeYinshTurnActionStruct (Variables|Default|GetCurrentTurn) (Utilities|Array|MakeArray (Utilities|Struct|MakeYinshSpaceActionStruct "NewEnumerator1" (Utilities|Struct|MakeYinshSpaceStruct (LocalVariables|GetLocalVinshSpace) (Variables|/Game/Yinsh/Widgets/WBP_YinshSpace.WBP_YinshSpace_C|GetLetterAxis (LocalVariables|GetLocalVinshSpace)) (Variables|/Game/Yinsh/Widgets/WBP_YinshSpace.WBP_YinshSpace_C|GetNumberAxis (LocalVariables|GetLocalVinshSpace)))) (Utilities|Struct|MakeYinshSpaceActionStruct "NewEnumerator4" (Utilities|Struct|MakeYinshSpaceStruct _output (Variables|/Game/Yinsh/Widgets/WBP_YinshSpace.WBP_YinshSpace_C|GetLetterAxis _output) (Variables|/Game/Yinsh/Widgets/WBP_YinshSpace.WBP_YinshSpace_C|GetNumberAxis _output))))))
                              (return)))))))))
              (:else))))))))

(fn OnConfirmMove
  (bind _currentturn (Variables|Default|GetCurrentTurn))
  (bind _whiteannulusdeployed (Variables|Default|GetWhiteAnnulusDeployed))
  (bind _blackannulusdeployed (Variables|Default|GetBlackAnnulusDeployed))
  (bind _returnvalue (Utilities|Select :Index _currentturn :NewEnumerator0 _whiteannulusdeployed :NewEnumerator1 _blackannulusdeployed))
  (if (== (Utilities|Array|Length (Variables|Default|GetSelectedSpaceArray)) (select (Variables|Default|GetbDeployPhaseOver) 2 1))
    (Utilities|FlowControl|Sequence
      (:then_0
        (if (and (Utilities|Enum|Equal(Enum) (Variables|Default|GetCurrentTurn) "NewEnumerator1") (== (Variables|Default|GetBlackAnnulusDeployed) 4))
          (Variables|Default|SetbDeployPhaseOver true)))
      (:then_1
        (Utilities|FlowControl|Sequence
          (:then_0
            (if (< _returnvalue 5)
              (Math|Integer|IncrementInt _returnvalue)))
          (:then_1
            (Utilities|Array|Add (Variables|Default|GetTurnActionArray) (Variables|Default|GetCurrentTurnAction))
            (CallFunction|SetCurrentTurn (Utilities|Select :Index (Variables|Default|GetCurrentTurn) :NewEnumerator0 "NewEnumerator1" :NewEnumerator1 "NewEnumerator0"))
            (Variables|Default|SetCurrentTurnAction "")
            (Utilities|Array|Clear (Variables|Default|GetSelectedSpaceArray))))))
    (else
      (return))))

(fn IsValidAnnulusMove
  (params (Annulus :type WBP%20Yinsh%20Space%20Object%20Reference) (MoveDestination :type WBP%20Yinsh%20Space%20Object%20Reference))
  (LocalVariables|SetLocalAnnulus Annulus)
  (Development|PrintString (Utilities|GetDisplayName MoveDestination))
  (LocalVariables|SetLocalMoveDestination MoveDestination)
  (LocalVariables|SetbAlongLetterAxis (Utilities|Enum|Equal(Enum) (Variables|/Game/Yinsh/Widgets/WBP_YinshSpace.WBP_YinshSpace_C|GetLetterAxis (LocalVariables|GetLocalMoveDestination)) (Variables|/Game/Yinsh/Widgets/WBP_YinshSpace.WBP_YinshSpace_C|GetLetterAxis (LocalVariables|GetLocalAnnulus))))
  (LocalVariables|SetbAlongNumberAxis (== (Variables|/Game/Yinsh/Widgets/WBP_YinshSpace.WBP_YinshSpace_C|GetNumberAxis (LocalVariables|GetLocalAnnulus)) (Variables|/Game/Yinsh/Widgets/WBP_YinshSpace.WBP_YinshSpace_C|GetNumberAxis (LocalVariables|GetLocalMoveDestination))))
  (LocalVariables|SetbAlongDiagonal (== (- (Math|Conversions|ToInteger(Byte) (Variables|/Game/Yinsh/Widgets/WBP_YinshSpace.WBP_YinshSpace_C|GetLetterAxis (LocalVariables|GetLocalMoveDestination))) (Math|Conversions|ToInteger(Byte) (Variables|/Game/Yinsh/Widgets/WBP_YinshSpace.WBP_YinshSpace_C|GetLetterAxis (LocalVariables|GetLocalAnnulus)))) (- (Variables|/Game/Yinsh/Widgets/WBP_YinshSpace.WBP_YinshSpace_C|GetNumberAxis (LocalVariables|GetLocalMoveDestination)) (Variables|/Game/Yinsh/Widgets/WBP_YinshSpace.WBP_YinshSpace_C|GetNumberAxis (LocalVariables|GetLocalAnnulus)))))
  (if (not (Math|Boolean|ORBoolean (LocalVariables|GetbAlongLetterAxis) (LocalVariables|GetbAlongNumberAxis) (LocalVariables|GetbAlongDiagonal)))
    (return false)
    (else
      (Utilities|FlowControl|Sequence
        (:then_0
          (if (LocalVariables|GetbAlongLetterAxis)
            (LocalVariables|SetLocalIndex (Variables|/Game/Yinsh/Widgets/WBP_YinshSpace.WBP_YinshSpace_C|GetNumberAxis (LocalVariables|GetLocalAnnulus)))
            (while (!= (LocalVariables|GetLocalIndex) (- (Variables|/Game/Yinsh/Widgets/WBP_YinshSpace.WBP_YinshSpace_C|GetNumberAxis (LocalVariables|GetLocalMoveDestination)) 1))
              (bind _output_get (LocalVariables|SetLocalIndex (+ (LocalVariables|GetLocalIndex) (Class|KismetMathLibrary|SignOfInteger (- (- (Variables|/Game/Yinsh/Widgets/WBP_YinshSpace.WBP_YinshSpace_C|GetNumberAxis (LocalVariables|GetLocalMoveDestination)) 1) (- (Variables|/Game/Yinsh/Widgets/WBP_YinshSpace.WBP_YinshSpace_C|GetNumberAxis (LocalVariables|GetLocalAnnulus)) 1))))))
              (Utilities|IsValid (CallFunction|GetYinshSpace (Variables|/Game/Yinsh/Widgets/WBP_YinshSpace.WBP_YinshSpace_C|GetLetterAxis (LocalVariables|GetLocalAnnulus)) _output_get)
                (:Is%20Valid
                  (switch Utilities|FlowControl|Switch|SwitchonYinshSpaceState (Variables|/Game/Yinsh/Widgets/WBP_YinshSpace.WBP_YinshSpace_C|GetSpaceState (CallFunction|GetYinshSpace (Variables|/Game/Yinsh/Widgets/WBP_YinshSpace.WBP_YinshSpace_C|GetLetterAxis (LocalVariables|GetLocalAnnulus)) _output_get))
                    (:NewEnumerator0
                      (if (LocalVariables|GetbSawSpirit)
                        (return (== (Math|Conversions|ToInteger(Byte) (Variables|/Game/Yinsh/Widgets/WBP_YinshSpace.WBP_YinshSpace_C|GetLetterAxis (LocalVariables|GetLocalMoveDestination))) (LocalVariables|GetLocalIndex)))))
                    (:NewEnumerator1
                      (if (!= (CallFunction|GetYinshSpace (Variables|/Game/Yinsh/Widgets/WBP_YinshSpace.WBP_YinshSpace_C|GetLetterAxis (LocalVariables|GetLocalAnnulus)) _output_get) (LocalVariables|GetLocalAnnulus))
                        (Utilities|IsBlockingSpacethePreview (CallFunction|GetYinshSpace (Variables|/Game/Yinsh/Widgets/WBP_YinshSpace.WBP_YinshSpace_C|GetLetterAxis (LocalVariables|GetLocalAnnulus)) _output_get)
                          (:else
                            (return false)))))
                    (:NewEnumerator2
                      (LocalVariables|SetbSawSpirit true))
                    (:NewEnumerator4
                      (if (!= (CallFunction|GetYinshSpace (Variables|/Game/Yinsh/Widgets/WBP_YinshSpace.WBP_YinshSpace_C|GetLetterAxis (LocalVariables|GetLocalAnnulus)) _output_get) (LocalVariables|GetLocalAnnulus))
                        (Utilities|IsBlockingSpacethePreview (CallFunction|GetYinshSpace (Variables|/Game/Yinsh/Widgets/WBP_YinshSpace.WBP_YinshSpace_C|GetLetterAxis (LocalVariables|GetLocalAnnulus)) _output_get)
                          (:else
                            (return false)))))
                    (:NewEnumerator5
                      (LocalVariables|SetbSawSpirit true))))))))
        (:then_1
          (if (LocalVariables|GetbAlongNumberAxis)
            (LocalVariables|SetLocalIndex (Math|Conversions|ToInteger(Byte) (Variables|/Game/Yinsh/Widgets/WBP_YinshSpace.WBP_YinshSpace_C|GetLetterAxis (LocalVariables|GetLocalAnnulus))))
            (while (!= (LocalVariables|GetLocalIndex) (Math|Conversions|ToInteger(Byte) (Variables|/Game/Yinsh/Widgets/WBP_YinshSpace.WBP_YinshSpace_C|GetLetterAxis (LocalVariables|GetLocalMoveDestination))))
              (bind _output_get_2 (LocalVariables|SetLocalIndex (+ (LocalVariables|GetLocalIndex) (Class|KismetMathLibrary|SignOfInteger (- (Math|Conversions|ToInteger(Byte) (Variables|/Game/Yinsh/Widgets/WBP_YinshSpace.WBP_YinshSpace_C|GetLetterAxis (LocalVariables|GetLocalMoveDestination))) (Math|Conversions|ToInteger(Byte) (Variables|/Game/Yinsh/Widgets/WBP_YinshSpace.WBP_YinshSpace_C|GetLetterAxis (LocalVariables|GetLocalAnnulus))))))))
              (Utilities|IsValid (CallFunction|GetYinshSpace (Utilities|Enum|ByteToEnumYinshLetterAxis (Math|Conversions|ToByte(Integer) _output_get_2)) (Variables|/Game/Yinsh/Widgets/WBP_YinshSpace.WBP_YinshSpace_C|GetNumberAxis (LocalVariables|GetLocalAnnulus)))
                (:Is%20Valid
                  (switch Utilities|FlowControl|Switch|SwitchonYinshSpaceState (Variables|/Game/Yinsh/Widgets/WBP_YinshSpace.WBP_YinshSpace_C|GetSpaceState (CallFunction|GetYinshSpace (Utilities|Enum|ByteToEnumYinshLetterAxis (Math|Conversions|ToByte(Integer) _output_get_2)) (Variables|/Game/Yinsh/Widgets/WBP_YinshSpace.WBP_YinshSpace_C|GetNumberAxis (LocalVariables|GetLocalAnnulus))))
                    (:NewEnumerator0
                      (if (LocalVariables|GetbSawSpirit)
                        (return (== (Math|Conversions|ToInteger(Byte) (Variables|/Game/Yinsh/Widgets/WBP_YinshSpace.WBP_YinshSpace_C|GetLetterAxis (LocalVariables|GetLocalMoveDestination))) (LocalVariables|GetLocalIndex)))))
                    (:NewEnumerator1
                      (Utilities|IsBlockingSpacethePreview (CallFunction|GetYinshSpace (Utilities|Enum|ByteToEnumYinshLetterAxis (Math|Conversions|ToByte(Integer) _output_get_2)) (Variables|/Game/Yinsh/Widgets/WBP_YinshSpace.WBP_YinshSpace_C|GetNumberAxis (LocalVariables|GetLocalAnnulus)))
                        (:else
                          (return false))))
                    (:NewEnumerator2
                      (LocalVariables|SetbSawSpirit true))
                    (:NewEnumerator4
                      (Utilities|IsBlockingSpacethePreview
                        (:else
                          (return false))))
                    (:NewEnumerator5
                      (LocalVariables|SetbSawSpirit true))))))))
        (:then_2
          (if (LocalVariables|GetbAlongDiagonal)
            (for _index (range 1 (- (Variables|/Game/Yinsh/Widgets/WBP_YinshSpace.WBP_YinshSpace_C|GetNumberAxis (LocalVariables|GetLocalMoveDestination)) (Variables|/Game/Yinsh/Widgets/WBP_YinshSpace.WBP_YinshSpace_C|GetNumberAxis (LocalVariables|GetLocalAnnulus))))
              (LocalVariables|SetLocalIndex _index)
              (Utilities|IsValid (CallFunction|GetYinshSpace (Utilities|Enum|ByteToEnumYinshLetterAxis (Math|Conversions|ToByte(Integer) (+ (Math|Conversions|ToInteger(Byte) (Variables|/Game/Yinsh/Widgets/WBP_YinshSpace.WBP_YinshSpace_C|GetLetterAxis (LocalVariables|GetLocalAnnulus))) _index))) (+ (Variables|/Game/Yinsh/Widgets/WBP_YinshSpace.WBP_YinshSpace_C|GetNumberAxis (LocalVariables|GetLocalAnnulus)) _index))
                (:Is%20Valid
                  (switch Utilities|FlowControl|Switch|SwitchonYinshSpaceState (Variables|/Game/Yinsh/Widgets/WBP_YinshSpace.WBP_YinshSpace_C|GetSpaceState (CallFunction|GetYinshSpace (Utilities|Enum|ByteToEnumYinshLetterAxis (Math|Conversions|ToByte(Integer) (+ (Math|Conversions|ToInteger(Byte) (Variables|/Game/Yinsh/Widgets/WBP_YinshSpace.WBP_YinshSpace_C|GetLetterAxis (LocalVariables|GetLocalAnnulus))) _index))) (+ (Variables|/Game/Yinsh/Widgets/WBP_YinshSpace.WBP_YinshSpace_C|GetNumberAxis (LocalVariables|GetLocalAnnulus)) _index)))
                    (:NewEnumerator0
                      (if (LocalVariables|GetbSawSpirit)
                        (return (== (- (Variables|/Game/Yinsh/Widgets/WBP_YinshSpace.WBP_YinshSpace_C|GetNumberAxis (LocalVariables|GetLocalMoveDestination)) (Variables|/Game/Yinsh/Widgets/WBP_YinshSpace.WBP_YinshSpace_C|GetNumberAxis (LocalVariables|GetLocalAnnulus))) (LocalVariables|GetLocalIndex)))))
                    (:NewEnumerator1
                      (Utilities|IsBlockingSpacethePreview (CallFunction|GetYinshSpace (Utilities|Enum|ByteToEnumYinshLetterAxis (Math|Conversions|ToByte(Integer) (+ (Math|Conversions|ToInteger(Byte) (Variables|/Game/Yinsh/Widgets/WBP_YinshSpace.WBP_YinshSpace_C|GetLetterAxis (LocalVariables|GetLocalAnnulus))) _index))) (+ (Variables|/Game/Yinsh/Widgets/WBP_YinshSpace.WBP_YinshSpace_C|GetNumberAxis (LocalVariables|GetLocalAnnulus)) _index))
                        (:else
                          (return false))))
                    (:NewEnumerator2
                      (LocalVariables|SetbSawSpirit true))
                    (:NewEnumerator4
                      (Utilities|IsBlockingSpacethePreview (CallFunction|GetYinshSpace (Utilities|Enum|ByteToEnumYinshLetterAxis (Math|Conversions|ToByte(Integer) (+ (Math|Conversions|ToInteger(Byte) (Variables|/Game/Yinsh/Widgets/WBP_YinshSpace.WBP_YinshSpace_C|GetLetterAxis (LocalVariables|GetLocalAnnulus))) _index))) (+ (Variables|/Game/Yinsh/Widgets/WBP_YinshSpace.WBP_YinshSpace_C|GetNumberAxis (LocalVariables|GetLocalAnnulus)) _index))
                        (:else
                          (return false))))
                    (:NewEnumerator5
                      (LocalVariables|SetbSawSpirit true))))))))
        (:then_3
          (return true))))))

(fn GetYinshSpace
  (params (LetterAxis :type YinshLetterAxis%20Enum :default "NewEnumerator0") (NumberAxis :type Integer))
  (bind _yinshmap (Variables|Default|GetYinshMap))
  (bind (_value _returnvalue) (Utilities|Map|Find _yinshmap LetterAxis))
  (if _returnvalue
    (return (Utilities|Array|Get(acopy) (Utilities|Struct|BreakYinshRow _value) (- NumberAxis 1)))
    (else
      (return 0))))